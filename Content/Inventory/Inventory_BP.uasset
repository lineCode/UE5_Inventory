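; Inventory Blueprint that owns an Inventory object and provides both slot-based and list-based UI for it.
; BeginPlay constructs the Inventory and sizes its cell array to the configured cell count.
; Each UI variant has separate events to create its viewport widget and bind to Inventory delegates, though none are called from BeginPlay.
; Cell updates refresh only the affected cell widget, while inventory updates remove and recreate the whole widget.
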(event `self.ReceiveBeginPlay`
  (bind _returnvalue (`|GenericCreateObject` "/Script/UE5_Inventory.Inventory" (`self.Amount Of Cells`)))
  (bind _output_get (set `self.Inventory` _returnvalue))
  (bind _returnvalue_2 (`Inventory.GetAmountOfCells` _output_get))
  (if (> _returnvalue_2 0)
    (`KismetArrayLibrary.Array_Resize` (`Inventory.Cells` _output_get) _returnvalue_2)))

(event `CreateWidget`
  ;[1 1 1] Slot-based inventory
  (bind _returnvalue (`|CreateWidget` "/Game/Inventory/Slot-basedInventory/Widgets/MainSlotBasedInventoryWidget.MainSlotBasedInventoryWidget_C" null (`self.Inventory`) 5))
  (bind _output_get (set `self.MainSlotBasedWidget` _returnvalue))
  (set `/Game/Inventory/Slot-basedInventory/Widgets/MainSlotBasedInventoryWidget.InventoryWidget` (`/Game/Inventory/Slot-basedInventory/Widgets/MainSlotBasedInventoryWidget.InventoryWidget` _output_get) _output_get)
  (`UserWidget.AddToViewport` (`self.MainSlotBasedWidget`) 0))

(event `PerformBinds`
  (bind _inventory (`self.Inventory`))
  ;[1 1 1] Slot-based inventory
  (add `Inventory.OnCellUpdated` _inventory (`|CreateDelegate` :!event `OnCellUpdated`))
  (add `Inventory.OnInventoryUpdated` _inventory (`|CreateDelegate` :!event `OnInventoryUpdated`)))

(event `OnCellUpdated`
  (params (CellToUpdate :type Integer))
  ;[1 1 1] Slot-based inventory
  (`/Game/Inventory/Slot-basedInventory/Widgets/InventorySlot.UpdateCell` (`|GetArrayItem` (`/Game/Inventory/Slot-basedInventory/Widgets/Slot-Based_Inventory_Widget.CellsWidget` (`/Game/Inventory/Slot-basedInventory/Widgets/MainSlotBasedInventoryWidget.InventoryWidget` (`self.MainSlotBasedWidget`))) CellToUpdate)))

(event `OnInventoryUpdated`
  ;[1 1 1] Slot-based inventory
  (`/Engine/EditorBlueprintResources/StandardMacros.IsValid` (`self.MainSlotBasedWidget`)
    (:`Is Valid`
      (`/Engine/EditorBlueprintResources/StandardMacros.IsValid` (`self.Inventory`)
        (:`Is Valid`
          (`Widget.RemoveFromParent` (`self.MainSlotBasedWidget`))
          (set `self.MainSlotBasedWidget` null)
          (`self.CreateWidget`))))))

(event `CreateWidget_2`
  ;[1 1 1] List-based inventory
  (bind _returnvalue (`|CreateWidget` "/Game/Inventory/List-basedInventory/MainListBasedInventoryWidget.MainListBasedInventoryWidget_C" null (`self.Inventory`)))
  (bind _output_get (set `self.MainListBasedWidget` _returnvalue))
  (set `/Game/Inventory/List-basedInventory/MainListBasedInventoryWidget.InventoryWidget` (`/Game/Inventory/List-basedInventory/MainListBasedInventoryWidget.InventoryWidget` _output_get) _output_get)
  (`UserWidget.AddToViewport` (`self.MainListBasedWidget`) 0))

(event `PerformBinds_2`
  (bind _inventory (`self.Inventory`))
  ;[1 1 1] List-based inventory
  (add `Inventory.OnCellUpdated` _inventory (`|CreateDelegate` :!event `OnCellUpdated_2`))
  (add `Inventory.OnInventoryUpdated` _inventory (`|CreateDelegate` :!event `OnInventoryUpdated_2`)))

(event `OnCellUpdated_2`
  (params (CellToUpdate :type Integer))
  (bind _output (`|GetArrayItem` (`/Game/Inventory/List-basedInventory/ListBasedInventoryWidget.CellsWidget` (`/Game/Inventory/List-basedInventory/MainListBasedInventoryWidget.InventoryWidget` (`self.MainListBasedWidget`))) CellToUpdate))
  ;[1 1 1] List-based inventory
  (`/Engine/EditorBlueprintResources/StandardMacros.IsValid` _output
    (:`Is Valid`
      (`/Game/Inventory/List-basedInventory/CellWidget.UpdateCell` _output))))

(event `OnInventoryUpdated_2`
  (bind _mainlistbasedwidget (`self.MainListBasedWidget`))
  ;[1 1 1] List-based inventory
  (`self.DestroyWidgets` _mainlistbasedwidget)
  (`self.SetToNull` _mainlistbasedwidget)
  (`self.CreateWidget_2`))

(fn `DestroyWidgets`
  (params (TargetWidget :type "UserWidget Object Reference"))
  (`/Engine/EditorBlueprintResources/StandardMacros.IsValid` TargetWidget
    (:`Is Valid`
      (`Widget.RemoveFromParent` TargetWidget))
    (:`Is Not Valid`
      _))
  (return))