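; BP_PickUpActor is a world pickup that adds an item to the top-down character's slot-based inventory on sphere overlap.
; It passes its configured item class and amount to the inventory's AddItemNew, then refreshes every cell in the character's inventory widget.
; On success, any leftover amount stays on the pickup for later collection, and the actor destroys itself when nothing remains.
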(event `self.Sphere.OnComponentBeginOverlap`
  (params (OverlappedComponent :type "PrimitiveComponent Object Reference") (OtherActor :type "Actor Object Reference") (OtherComp :type "PrimitiveComponent Object Reference") (OtherBodyIndex :type Integer) (bFromSweep :type Boolean) (SweepResult :type "HitResult Structure (by ref)"))
  (bind _asbp_top_down_character (cast `/Game/TopDown/Blueprints/BP_TopDownCharacter` OtherActor))
  (bind (_issuccess _rest) (`Inventory.AddItemNew` (`/Game/TopDown/Blueprints/BP_TopDownCharacter.Inventory` _asbp_top_down_character) (defaults `Object` (`self.ItemToAdd`)) (`self.Amount`)))
  (`self.UpdateInventory` _asbp_top_down_character)
  (if _issuccess
    (if (> _rest 0)
      (set `self.Amount` _rest)
      (else
        (`self.K2_DestroyActor`)))))

(fn `UpdateInventory`
  (params (Character :type "/Game/TopDown/Blueprints/BP_TopDownCharacter Object Reference"))
  (for _array_element (`/Game/Inventory/Slot-basedInventory/Widgets/Slot-Based_Inventory_Widget.CellsWidget` (`/Game/Inventory/Slot-basedInventory/Widgets/MainInventoryWidget.InventoryWidget` (`/Game/TopDown/Blueprints/BP_TopDownCharacter.MainWidget` Character)))
    (`/Game/Inventory/Slot-basedInventory/Widgets/InventorySlot.UpdateSlot` _array_element)))

(fn `UserConstructionScript`)