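; Slot-based inventory Blueprint that stores items as class and amount pairs in a fixed-size Cells array and creates the on-screen inventory widget at BeginPlay.
; AddItem reads Stackable from item class defaults, filling the first partial stack or empty slot, or placing non-stackables one per slot.
; It recurses on overflow, returning any unplaced Rest, and refreshes each changed cell's widget by index.
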(event `self.ReceiveBeginPlay`
  (`KismetArrayLibrary.Array_Resize` (`self.Cells`) (`self.AmountOfCells`))
  (bind _returnvalue (`|CreateWidget` "/Game/Inventory/Slot-basedInventory/MainInventoryWidget.MainInventoryWidget_C" null self (`self.Cells Per Row`)))
  (bind _output_get (set `self.MainWidget` _returnvalue))
  (set `self.Inventory Widget` (`/Game/Inventory/Slot-basedInventory/MainInventoryWidget.InventoryWidget` _output_get))
  (`UserWidget.AddToViewport` (`self.MainWidget`) 0))

(event `UpdateCellAtIndex`
  (params (Index :type Integer))
  (`/Game/Inventory/Slot-basedInventory/InventorySlot.UpdateSlot` (`|GetArrayItem` (`/Game/Inventory/Slot-basedInventory/Slot-Based_Inventory_Widget.CellsWidget` (`self.Inventory Widget`)) Index)))

(fn `AddItem`
  (params (ItemClass :type "/Game/Inventory/Slot-basedInventory/ItemClasses/BP_MasterItem Class Reference") (Amount :type Integer))
  (returns (IsSuccess :type Boolean) (Rest :type Integer))
  (locals (ItemLocal :type "/Game/Inventory/Slot-basedInventory/ItemClasses/BP_MasterItem Class Reference") (AmountLocal :type Integer) (FoundIndex :type Integer))
  (bind _amountlocal (`local.AmountLocal`))
  (bind (_output_itemclass _output_amount) (break `/Game/Inventory/Slot-basedInventory/Structures/InventoryCellStruct` (`|GetArrayItem` (`self.Cells`) (`local.FoundIndex`))))
  (bind _returnvalue (+ _output_amount (`local.AmountLocal`)))
  (set `local.ItemLocal` ItemClass)
  (set `local.AmountLocal` Amount)
  (if (`.Stackable_14_EB33C7034E5477C9A91F14BDBA8D933E` (break `/Game/Inventory/Slot-basedInventory/Structures/ItemInfoStruct` (defaults `Object` ItemClass)))
    (bind (_issuccess _index) (`self.SearchFreeStack` (`local.ItemLocal`)))
    (if _issuccess
      (set `local.FoundIndex` _index)
      (if (> _returnvalue (`self.MaxStackSize`))
        (set `local.AmountLocal` (- _returnvalue (`self.MaxStackSize`)))
        (`KismetArrayLibrary.Array_Set` (`self.Cells`) (`local.FoundIndex`) (make `/Game/Inventory/Slot-basedInventory/Structures/InventoryCellStruct` (`local.ItemLocal`) (`self.MaxStackSize`)))
        (`self.UpdateCellAtIndex` (`local.FoundIndex`))
        (bind (_issuccess_2 _rest) (`self.AddItem` (`local.ItemLocal`) (`local.AmountLocal`)))
        (return true _rest)
        (else
          (`KismetArrayLibrary.Array_Set` (`self.Cells`) (`local.FoundIndex`) (make `/Game/Inventory/Slot-basedInventory/Structures/InventoryCellStruct` (`local.ItemLocal`) _returnvalue))
          (`self.UpdateCellAtIndex` (`local.FoundIndex`))
          (return true 0)))
      (else
        (bind (_issuccess_3 _index_2) (`self.SearchEmptySlot`))
        (if _issuccess_3
          (set `local.FoundIndex` _index_2)
          (if (> (`local.AmountLocal`) (`self.MaxStackSize`))
            (`KismetArrayLibrary.Array_Set` (`self.Cells`) (`local.FoundIndex`) (make `/Game/Inventory/Slot-basedInventory/Structures/InventoryCellStruct` (`local.ItemLocal`) (`self.MaxStackSize`)))
            (`self.UpdateCellAtIndex` (`local.FoundIndex`))
            (bind (_issuccess_4 _rest_2) (`self.AddItem` (`local.ItemLocal`) (- (`local.AmountLocal`) (`self.MaxStackSize`))))
            (return true _rest_2)
            (else
              (`KismetArrayLibrary.Array_Set` (`self.Cells`) (`local.FoundIndex`) (make `/Game/Inventory/Slot-basedInventory/Structures/InventoryCellStruct` (`local.ItemLocal`) (`local.AmountLocal`)))
              (`self.UpdateCellAtIndex` (`local.FoundIndex`))
              (return true 0)))
          (else
            (return false (`local.AmountLocal`))))))
    (else
      (bind (_issuccess_5 _index_3) (`self.SearchEmptySlot`))
      (if _issuccess_5
        (bind _output_get (set `local.FoundIndex` _index_3))
        (`KismetArrayLibrary.Array_Set` (`self.Cells`) _output_get (make `/Game/Inventory/Slot-basedInventory/Structures/InventoryCellStruct` (`local.ItemLocal`) 1))
        (`self.UpdateCellAtIndex` (`local.FoundIndex`))
        (if (> _amountlocal 1)
          (bind (_issuccess_6 _rest_3) (`self.AddItem` (`local.ItemLocal`) (- _amountlocal 1)))
          (return true _rest_3)
          (else
            (return true 0)))
        (else
          (return false (`local.AmountLocal`)))))))

(fn `GetAmountAtIndex`
  (params (Index :type Integer))
  (returns (Amount :type Integer))
  (bind (_output_itemclass _output_amount) (break `/Game/Inventory/Slot-basedInventory/Structures/InventoryCellStruct` (`|GetArrayItem` (`self.Cells`) Index)))
  (return _output_amount))

(fn `GetItemInfoAtIndex`
  (params (Index :type Integer))
  (returns (IsCellEmpty :type Boolean) (ItemInfo :type "/Game/Inventory/Slot-basedInventory/Structures/ItemInfoStruct Structure") (Amount :type Integer))
  (bind (_output_itemclass _output_amount) (break `/Game/Inventory/Slot-basedInventory/Structures/InventoryCellStruct` (`|GetArrayItem` (`self.Cells`) Index)))
  (if (`KismetSystemLibrary.IsValidClass` _output_itemclass)
    (return false (defaults `Object` _output_itemclass) _output_amount)
    (else
      (return true (struct) 0))))

(fn `IsSlotEmpty`
  (params (Index :type Integer))
  (returns (IsEmpty :type Boolean))
  (bind _output_itemclass (break `/Game/Inventory/Slot-basedInventory/Structures/InventoryCellStruct` (`|GetArrayItem` (`self.Cells`) Index)))
  (return (not (`KismetSystemLibrary.IsValidClass` _output_itemclass))))

(fn `SearchEmptySlot`
  (returns (IsSuccess :type Boolean) (Index :type Integer))
  (locals (BoolLocal :type Boolean) (IndexLocal :type Integer))
  (for (_array_element _array_index) (`self.Cells`)
    (if (not (`KismetSystemLibrary.IsValidClass` (`.ItemClass_3_EA93989D4FC16A73059B319D91710E88` (break `/Game/Inventory/Slot-basedInventory/Structures/InventoryCellStruct` _array_element))))
      (set `local.BoolLocal` true)
      (set `local.IndexLocal` _array_index)
      (break)))
  (return (`local.BoolLocal`) (`local.IndexLocal`)))

(fn `SearchFreeStack`
  (params (ItemClass :type "/Game/Inventory/Slot-basedInventory/ItemClasses/BP_MasterItem Class Reference"))
  (returns (IsSuccess :type Boolean) (Index :type Integer))
  (locals (BoolLocal :type Boolean) (IndexLocal :type Integer))
  (for (_array_element _array_index) (`self.Cells`)
    (bind (_itemclass _amount) (break `/Game/Inventory/Slot-basedInventory/Structures/InventoryCellStruct` _array_element))
    (if (`KismetSystemLibrary.IsValidClass` _itemclass)
      (if (and (== _itemclass ItemClass) (< _amount (`self.MaxStackSize`)))
        (set `local.BoolLocal` true)
        (set `local.IndexLocal` _array_index)
        (break))))
  (return (`local.BoolLocal`) (`local.IndexLocal`)))

(fn `UserConstructionScript`)